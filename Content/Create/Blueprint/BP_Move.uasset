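; BP_Move is an actor that slides its static mesh back and forth along the local X axis.
; Each Tick steps a position value by a fixed amount and applies it as the mesh's relative X location.
; A boolean flips the direction when the value passes either end of a fixed range, so motion speed depends on frame rate rather than delta time.
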(event `self.ReceiveTick`
  (params (DeltaSeconds :type "Float (single-precision)"))
  (if (`self.Ture / Fales`)
    (bind _output_get (set `self.Value` (+ (`self.Value`) 10.0)))
    (`SceneComponent.K2_SetRelativeLocation` (`self.StaticMesh`) (`KismetMathLibrary.MakeVector` _output_get) false false)
    (if (> (`self.Value`) 200.0)
      (set `self.Ture / Fales` false))
    (else
      (bind _output_get_2 (set `self.Value` (+ (`self.Value`) -10.0)))
      (`SceneComponent.K2_SetRelativeLocation` (`self.StaticMesh`) (`KismetMathLibrary.MakeVector` _output_get_2) false false)
      (if (< (`self.Value`) 0.0)
        (set `self.Ture / Fales` true)))))

(fn `UserConstructionScript`)