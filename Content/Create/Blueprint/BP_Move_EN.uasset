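; BP_Move_EN is an actor that moves its static mesh around a square loop in the relative XZ plane.
; Each Tick switches on the MoveType enum, steps XValue or ZValue by a fixed amount and applies it as the mesh's relative location.
; Crossing a boundary advances the state through Right, Up, Left and Down, with a per-frame step that ignores delta time, so speed depends on frame rate.
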(event `self.ReceiveTick`
  (params (DeltaSeconds :type "Float (single-precision)"))
  (switch `/Game/Create/Blueprint/EN_Move_Type` (`self.Move_Type`)
    (:`NewEnumerator0`
      (bind _output_get (set `self.X_Value` (+ (`self.X_Value`) 5.0)))
      (`SceneComponent.K2_SetRelativeLocation` (`self.StaticMesh`) (`KismetMathLibrary.MakeVector` _output_get 0.0 (`self.Z_Value`)) false false)
      (if (> (`self.X_Value`) 300.0)
        (set `self.Move_Type` "NewEnumerator1")))
    (:`NewEnumerator1`
      (bind _output_get_2 (set `self.Z_Value` (+ (`self.Z_Value`) 5.0)))
      (`SceneComponent.K2_SetRelativeLocation` (`self.StaticMesh`) (`KismetMathLibrary.MakeVector` (`self.X_Value`) 0.0 _output_get_2) false false)
      (if (> (`self.Z_Value`) 300.0)
        (set `self.Move_Type` "NewEnumerator2")))
    (:`NewEnumerator2`
      (bind _output_get_3 (set `self.X_Value` (+ (`self.X_Value`) -5.0)))
      (`SceneComponent.K2_SetRelativeLocation` (`self.StaticMesh`) (`KismetMathLibrary.MakeVector` _output_get_3 0.0 (`self.Z_Value`)) false false)
      (if (< (`self.X_Value`) 0.0)
        (set `self.Move_Type` "NewEnumerator3")))
    (:`NewEnumerator3`
      (bind _output_get_4 (set `self.Z_Value` (+ (`self.Z_Value`) -5.0)))
      (`SceneComponent.K2_SetRelativeLocation` (`self.StaticMesh`) (`KismetMathLibrary.MakeVector` (`self.X_Value`) 0.0 _output_get_4) false false)
      (if (< (`self.Z_Value`) 0.0)
        (set `self.Move_Type` "NewEnumerator0")))))

(fn `UserConstructionScript`)