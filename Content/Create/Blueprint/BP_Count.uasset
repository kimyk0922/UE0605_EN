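; BP_Count is a count-up clock Blueprint that shows elapsed time as minute:second on a TextRender component.
; Tick adds delta time scaled by ten to a running total, so the clock runs ten times faster than the game's delta time.
; Helper functions split the total into minutes and seconds, floor each and zero-pad single digits; minutes never wrap into hours.
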(event `self.ReceiveTick`
  (params (DeltaSeconds :type "Float (single-precision)"))
  (bind _output_get (set `self.Time_Text` (+ (`self.Time_Text`) (* DeltaSeconds 10.0))))
  (`TextRenderComponent.K2_SetText` (`self.TextRender`) (`KismetTextLibrary.Conv_StringToText` (`KismetStringLibrary.Concat_StrStr` (`self.Float_To_Str` (/ _output_get 60.0)) ":" (`self.Float_To_Str` (mod _output_get 60.0))))))

(fn `Float_To_Str`
  (params (Number :type "Float (double-precision)"))
  (returns (String :type String))
  (bind _returnvalue (`KismetMathLibrary.FFloor` Number))
  (if (< Number 10.0)
    (return (`KismetStringLibrary.Concat_StrStr` "0" (`KismetStringLibrary.Conv_IntToString` _returnvalue)))
    (else
      (return (`KismetStringLibrary.Conv_IntToString` _returnvalue)))))

(fn `UserConstructionScript`)